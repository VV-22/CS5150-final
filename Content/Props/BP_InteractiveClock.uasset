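; Interactive clock prop that plays a breaking sound when the player interacts with it.
; Interact prints the EventComponent's CanBeInteracted flag and, if true, plays ClockBreak at the actor's location.
; It then reports the interaction to the EventComponent and disables further interaction, making it one-shot.
; Nodes for playing the ClockFall level sequence are present but never run.
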(event `self.Interact`
  (bind _eventcomponent (`self.EventComponent`))
  (bind _canbeinteracted (`/Game/GameLogic/EventComponent.CanBeInteracted` (`self.EventComponent`)))
  (`KismetSystemLibrary.PrintString` (`KismetStringLibrary.Conv_BoolToString` _canbeinteracted))
  (if _canbeinteracted
    (`GameplayStatics.PlaySoundAtLocation` "/Game/Sound/ClockBreak.ClockBreak" (`self.K2_GetActorLocation`) (struct) 1.0 1.0 0.0 null null null null)
    (`/Game/GameLogic/EventComponent.Interacted` _eventcomponent self)
    (`/Game/GameLogic/EventComponent.Change Interatible Status` _eventcomponent false)))

(fn `UserConstructionScript`
  (`parent.UserConstructionScript`))