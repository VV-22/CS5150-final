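; Base AI controller for AI character variants that manages brain logic and exposes the current perception target.
; It starts the brain component's logic on BeginPlay and stops it on UnPossess.
; GetTargetData reads the current target from GAPerceptionComponent and, when valid, returns its owning actor and target cache.
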(event `self.ReceiveBeginPlay`
  (`parent.ReceiveBeginPlay`)
  (`BrainComponent.StartLogic` (`self.BrainComponent`)))

(event `self.ReceiveUnPossess`
  (params (UnpossessedPawn :type "Pawn Object Reference"))
  (`BrainComponent.StopLogic` (`self.BrainComponent`) ""))

(fn `GetTargetData`
  (returns (TargetActor :type "Actor Object Reference") (TargetCache :type "TargetCache Structure"))
  (locals (TargetComponent :type "GATargetComponent Object Reference"))
  (bind _targetcomponent (`local.TargetComponent`))
  (bind _output_get (set `local.TargetComponent` (`GAPerceptionComponent.GetCurrentTarget` (`self.GAPerceptionComponent`))))
  (`/Engine/EditorBlueprintResources/StandardMacros.IsValid` _output_get
    (:`Is Valid`
      (return (`ActorComponent.GetOwner` _targetcomponent) (`GATargetComponent.GetTargetCache` _targetcomponent)))
    (:`Is Not Valid`
      (return null))))

(fn `UserConstructionScript`
  (`parent.UserConstructionScript`))