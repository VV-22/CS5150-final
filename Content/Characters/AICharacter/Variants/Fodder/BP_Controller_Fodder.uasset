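; BP_Controller_Fodder is the controller for the Fodder AI character variant, randomly deciding when it switches to charging.
; On BeginPlay it runs the parent logic, then starts a looping one-second timer that rolls against ChanceOfCharging.
; The first successful roll sets Charging and clears the timer, and nothing in this Blueprint resets the flag or acts on it.
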(event `self.ReceiveBeginPlay`
  (`parent.ReceiveBeginPlay`)
  (bind _returnvalue (`KismetSystemLibrary.K2_SetTimerDelegate` (delegate `TestTo Charge`) 1.0 true))
  (set `self.ChargeTestTimer` _returnvalue))

(event `TestTo Charge`
  (if (`KismetMathLibrary.RandomBoolWithWeight` (`self.ChanceOfCharging`))
    (set `self.Charging` true)
    (`KismetSystemLibrary.K2_ClearAndInvalidateTimerHandle` (`self.ChargeTestTimer`))))

(fn `UserConstructionScript`
  (`parent.UserConstructionScript`))