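; BP_TargetController is the AI controller for the Target AI character.
; On possess it runs the BT_Target behavior tree and puts the character in the Passive state.
; Helper functions set Passive, Attack or Investigate by writing an E_AIState value to the Blackboard's state key.
; Only the Passive setter is called within this controller.
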(event `self.ReceivePossess`
  (params (PossessedPawn :type "Pawn Object Reference"))
  (`self.RunBehaviorTree` "/Game/Characters/AICharacter/Target/BT_Target.BT_Target")
  (`self.Set State as Passive`))

(fn `Set State as Attack`
  (`BlackboardComponent.SetValueAsEnum` (`self.Blackboard`) (`self.State Key Name`) (enumliteral `/Game/Characters/AICharacter/Target/Enum/E_AIState` "NewEnumerator1")))

(fn `Set State as Investigate`
  (`BlackboardComponent.SetValueAsEnum` (`self.Blackboard`) (`self.State Key Name`) (enumliteral `/Game/Characters/AICharacter/Target/Enum/E_AIState` "NewEnumerator3")))

(fn `Set State as Passive`
  (`BlackboardComponent.SetValueAsEnum` (`self.Blackboard`) (`self.State Key Name`) (enumliteral `/Game/Characters/AICharacter/Target/Enum/E_AIState` "NewEnumerator0")))

(fn `UserConstructionScript`)