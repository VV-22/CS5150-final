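; BP_Target is an AI character with a fear meter, counted toward the level's win condition.
; Tick writes Fear into a fear bar widget and turns it to face the player camera.
; On destruction it decrements the game mode's AI count and opens YouWinMap when none remain.
; Helper functions expose its patrol route and map a speed state, including a slow Fear state, to walk speed.
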(event `self.ReceiveTick`
  (params (DeltaSeconds :type "Float (single-precision)"))
  (bind _fear_bar_widget (`self.Fear Bar Widget`))
  (bind _aswb_fear_bar (cast `/Game/Characters/AICharacter/Target/WB_FearBar` (`WidgetComponent.GetWidget` (`self.Fear Bar Widget`))))
  (`ProgressBar.SetPercent` (`/Game/Characters/AICharacter/Target/WB_FearBar.FearBar` _aswb_fear_bar) (/ (`self.Fear`) 100.0))
  (`SceneComponent.K2_SetWorldRotation` _fear_bar_widget (`KismetMathLibrary.FindLookAtRotation` (`SceneComponent.K2_GetComponentLocation` _fear_bar_widget) (`SceneComponent.K2_GetComponentLocation` (`PlayerCameraManager.TransformComponent` (`GameplayStatics.GetPlayerCameraManager` 0)))) false false))

(event `self.ReceiveDestroyed`
  (bind _asbp_game_aigame_mode (cast `/Game/GameLogic/BP_GameAIGameMode` (`GameplayStatics.GetGameMode`)))
  (bind _aicount (`/Game/GameLogic/BP_GameAIGameMode.AICount` _asbp_game_aigame_mode))
  (set `/Game/GameLogic/BP_GameAIGameMode.AICount` (- _aicount 1) _asbp_game_aigame_mode)
  (if (== _aicount 0)
    (`GameplayStatics.OpenLevel` "YouWinMap")))

(fn `Get Patrol Route`
  (returns (`Patrol Route` :type "/Game/Characters/AICharacter/Target/BP_PatrolRoute Object Reference"))
  (return (`self.PatrolRoute`)))

(fn `SetMovementSpeed`
  (params (Speed :type "/Game/Characters/AICharacter/Target/Enum/E_MovementSpeed Enum" :default "NewEnumerator0"))
  (returns (SpeedValue :type "Float (double-precision)"))
  (bind _output_get (set `CharacterMovementComponent.MaxWalkSpeed` (select `/Game/Characters/AICharacter/Target/Enum/E_MovementSpeed` Speed :`NewEnumerator1` 200.0 :`NewEnumerator2` 400.0 :`NewEnumerator3` 50.0 :!type "Float (single-precision)") (`self.CharacterMovement`)))
  (return _output_get))

(fn `UserConstructionScript`)