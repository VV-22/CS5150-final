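; BP_Interactible is an interactible actor that raises the Fear of nearby BP_Target actors when its Interacted event fires.
; The event runs a sphere overlap at the actor's location, using variables for radius, object types and class filter.
; Each overlapped BP_Target gains a fixed amount of Fear, and debug prints show the radius and overlap count.
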(event `Interacted`
  (bind _interactionradius (`self.InteractionRadius`))
  (`KismetSystemLibrary.PrintString` (`KismetStringLibrary.Conv_DoubleToString` _interactionradius))
  (bind _outactors (`KismetSystemLibrary.SphereOverlapActors` (`self.K2_GetActorLocation`) _interactionradius (`self.InteractionObjectType`) (`self.InteractionClassFilter`)))
  (`KismetSystemLibrary.PrintString` (`KismetStringLibrary.Concat_StrStr` "Count : " (`KismetStringLibrary.Conv_IntToString` (`KismetArrayLibrary.Array_Length` _outactors))))
  (for _array_element _outactors
    (bind _asbp_target (cast `/Game/Characters/AICharacter/Target/BP_Target` _array_element))
    (set `/Game/Characters/AICharacter/Target/BP_Target.Fear` (+ (`/Game/Characters/AICharacter/Target/BP_Target.Fear` _asbp_target) 10.0) _asbp_target)))

(fn `UserConstructionScript`)